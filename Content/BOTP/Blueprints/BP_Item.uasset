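; BP_Item is a world pickup that offers its ItemObject to the inventory of any BP_ThirdPersonCharacter overlapping its Collision.
; On BeginPlay it fills a missing ItemObject through GetDefaultItemObject, which is empty in this Blueprint.
; A successful TryAddItem on the InventoryComponent destroys the actor, leaving the data in the item object.
; A failed add prints a no-room message and leaves the pickup in place.
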(event OnComponentBeginOverlap(collision)
  (params (OverlappedComponent :type Primitive%20Component%20Object%20Reference) (OtherActor :type Actor%20Object%20Reference) (OtherComp :type Primitive%20Component%20Object%20Reference) (OtherBodyIndex :type Integer) (bFromSweep :type Boolean) (SweepResult :type Hit%20Result%20Structure%20%28by%20ref%29))
  (bind _asbp_third_person_character (Utilities|Casting|CastToBP_ThirdPersonCharacter OtherActor))
  ;[1 0 0] Attempts to add item to inventory based on current space if successful then the physical item is destroyed while the needed data for that item is stored in the item object
  (bind _added (Default|TryAddItem (Variables|/Game/ThirdPerson/Blueprints/BP_ThirdPersonCharacter.BP_ThirdPersonCharacter_C|GetInventoryComponent _asbp_third_person_character) (Variables|Private|GetItemObject)))
  (if _added
    (Actor|DestroyActor)
    (else
      (Development|PrintString "NO ROOM" true true "(R=1.000000,G=0.838494,B=0.000000,A=1.000000)"))))

(event EventBeginPlay
  (if (not (Utilities|IsValid (Variables|Private|GetItemObject)))
    (bind _bp_itemobject (Private|GetDefaultItemObject))
    (Variables|Private|SetItemObject _bp_itemobject)))

(fn ConstructionScript)

(fn GetDefaultItemObject
  (return 0))