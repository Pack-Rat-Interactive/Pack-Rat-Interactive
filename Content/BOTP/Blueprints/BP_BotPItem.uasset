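; BP_BotPItem is a world item actor that holds an ItemObject for its data, apparently meant for inventory pickup.
; On BeginPlay it fills a missing ItemObject from GetDefaultItemObject, which returns no value here.
; Its collision overlap only casts to BP_ThirdPersonCharacter.
; The logic to add the item and destroy the actor, or print "NO ROOM", is disconnected, as is a hide-actor call.
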(event OnComponentBeginOverlap(collision)
  (params (OverlappedComponent :type Primitive%20Component%20Object%20Reference) (OtherActor :type Actor%20Object%20Reference) (OtherComp :type Primitive%20Component%20Object%20Reference) (OtherBodyIndex :type Integer) (bFromSweep :type Boolean) (SweepResult :type Hit%20Result%20Structure%20%28by%20ref%29))
  (Utilities|Casting|CastToBP_ThirdPersonCharacter OtherActor))

(event EventBeginPlay
  (if (not (Utilities|IsValid (Variables|Private|GetItemObject)))
    (bind _bp_itemobject (Private|GetDefaultItemObject))
    (Variables|Private|SetItemObject _bp_itemobject)))

(fn ConstructionScript)

(fn GetDefaultItemObject
  (return 0))